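; BP_Door is a labyrinth door that opens only when both a switch and a torch are activated.
; On BeginPlay it caches one BP_Interrupteur and one BP_Torche through GetActorOfClass.
; CheckStatement tests both Activate flags, prints a message and triggers opening, with OpenDoor destroying the door actor.
; It does not poll on Tick, and nothing in this Blueprint calls CheckStatement.
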(event Custom|Event%20CheckStatement
  (if (== (Variables|/Game/Le_Labyrinthe/Blueprints/BP_Interrupteur.BP_Interrupteur_C|GetActivate (Variables|Default|GetInterrupteur)) true)
    (if (== (Variables|/Game/Le_Labyrinthe/Blueprints/BP_Torche.BP_Torche_C|GetActivate (Variables|Default|GetTorch)) true)
      (Development|PrintText "Door Open")
      (CallFunction|EventOpenDoor))))

(event Custom|Event%20OpenDoor
  (Actor|DestroyActor))

(event EventBeginPlay
  (bind _returnvalue (Actor|GetActorOfClass "/Game/Le_Labyrinthe/Blueprints/BP_Torche.BP_Torche_C"))
  (Variables|Default|SetTorch _returnvalue)
  (bind _returnvalue_2 (Actor|GetActorOfClass "/Game/Le_Labyrinthe/Blueprints/BP_Interrupteur.BP_Interrupteur_C"))
  (Variables|Default|SetInterrupteur _returnvalue_2))

(event Collision|EventActorBeginOverlap
  (params (OtherActor :type Actor%20Object%20Reference)))

(event EventTick
  (params (DeltaSeconds :type Float%20%28single-precision%29)))

(fn ConstructionScript)